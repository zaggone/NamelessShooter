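; BP_NSBaseCharacter is a base character Blueprint that selects its mesh's animation Blueprint according to whether it is armed.
; On BeginPlay, SetAnimInstanceClass applies the class supplied by WeaponComponent when armed, otherwise it falls back to ABP_Unarmed.
; Tick and the construction script are empty, and a forward-vector debug line is left unconnected.
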(event EventBeginPlay
  (CallFunction|SetAnimInstanceClass))

(event Collision|EventActorBeginOverlap
  (params (OtherActor :type Actor%20Object%20Reference)))

(event EventTick
  (params (DeltaSeconds :type Float%20%28single-precision%29)))

(fn ConstructionScript)

(fn SetAnimInstanceClass
  (bind _weaponcomponent (Variables|Default|GetWeaponComponent))
  (bind _mesh (Variables|Character|GetMesh))
  (if (Variables|/Script/NamelessShooter.NSWeaponComponent|GetbArmed _weaponcomponent)
    (bind _returnvalue (Class|NSWeaponComponent|GetCurrentAnimInstanceClass _weaponcomponent))
    (Class|SkeletalMeshComponent|SetAnimClass _mesh _returnvalue)
    (else
      (Class|SkeletalMeshComponent|SetAnimClass _mesh "/Game/Animation/ABP_Unarmed.ABP_Unarmed_C"))))